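; Base room for procedural map generation that registers its size with BP_RoomManager and spawns neighboring rooms until pregeneration completes.
; It tries random rooms at a random number of door points (at least two), using collision-blocked spawning and next-tick retries up to a limit.
; Successful doors become valid teleports, and doors left untested go to the manager.
; The manager's wall event makes it spawn BP_BaseWall at each arrow position.
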(event `self.ReceiveBeginPlay`
  (bind _outitem (`KismetArrayLibrary.Array_Random` (`self.TestedDoorSpawns`)))
  (bind _returnvalue (`GameplayStatics.GetActorOfClass` "/Game/Tech/ProcGen/BP_RoomManager.BP_RoomManager_C")) ; Selects the Room Manager
  (bind _output_get (set `self.RoomManager Reference` _returnvalue))
  (add `/Game/Tech/ProcGen/BP_RoomManager.E_WallSpawn` _output_get (delegate `Activate Walls`))
  (message `/Game/Tech/ProcGen/BPI_RoomManager.Map Size Tracker` (`self.RoomManager Reference`) (`self.Room Size`) self) ; Sends Room Size and Type to RoomManager
  (`/Engine/EditorBlueprintResources/StandardMacros.DoOnce` false
    (:`Completed`
      (if (not (`/Game/Tech/ProcGen/BP_RoomManager.Map Pregen complete?` (`self.RoomManager Reference`)))
        (`KismetSystemLibrary.DelayUntilNextTick`)
        (for _ (range (`KismetMathLibrary.RandomIntegerInRange` 2 (`KismetArrayLibrary.Array_Length` (`self.TestedDoorSpawns`))))
          ;[1 1 1] Door Spawner
          (bind _returnvalue_2 (`|SpawnActorFromClass` (`KismetArrayLibrary.Array_Random` (`self.Rooms`)) (`KismetMathLibrary.Conv_VectorToTransform` (+ (* (`SceneComponent.GetForwardVector` _outitem) 2400.0) (`SceneComponent.K2_GetComponentLocation` _outitem))) "DontSpawnIfColliding" "OverrideRootScale" null null :!label _label)) ; Tries to spawn a Door
          (`/Engine/EditorBlueprintResources/StandardMacros.IsValid` _returnvalue_2
            (:`Is Valid`
              (`KismetArrayLibrary.Array_Add` (`self.ValidTeleports`) _outitem))
            (:`Is Not Valid`
              (bind _result (`/Engine/EditorBlueprintResources/StandardMacros.IncrementInt` (`self.Room Spawn Attempts`))
                (:`  `
                  (if (== _result (/ (`KismetArrayLibrary.Array_Length` (`self.Rooms`)) 2))
                    _
                    (else
                      (`KismetSystemLibrary.DelayUntilNextTick`)
                      (goto _label)))))))
          (`KismetArrayLibrary.Array_RemoveItem` (`self.TestedDoorSpawns`) _outitem))
        (`KismetSystemLibrary.DelayUntilNextTick`)
        (for _array_element (`self.TestedDoorSpawns`)
          (message `/Game/Tech/ProcGen/BPI_EmptyDoors.Door Data Sender` (`self.RoomManager Reference`) _array_element))))))

(event `Activate Walls`
  (`/Engine/EditorBlueprintResources/StandardMacros.DoOnce` false
    (:`Completed`
      (for _array_element (`self.ArrowPositions`)
        (bind _returnvalue (`SceneComponent.K2_GetComponentToWorld` _array_element))
        (`|SpawnActorFromClass` "/Game/Tech/ProcGen/Walls/BP_BaseWall.BP_BaseWall_C" (`KismetMathLibrary.MakeTransform` (.location _returnvalue) (`KismetMathLibrary.MakeRotator` 0.0 0.0 (.yaw (.rotation _returnvalue))) (.scale _returnvalue)) "AlwaysSpawn" "OverrideRootScale" null true null)))))

(fn `UserConstructionScript`)