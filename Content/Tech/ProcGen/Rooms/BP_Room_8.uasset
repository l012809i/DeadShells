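; BP_Room_8 is a procedural-generation room Blueprint that defines where its doors can spawn.
; Its construction script fills PossibleDoorSpawns with the room's ten DoorLocation references, then calls the parent construction script.
; The array is set before the parent call, and the event graph holds only disabled default events with no logic of its own.
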(fn `UserConstructionScript`
  ;[1 1 1] Set array of possible room positions
  (set `self.PossibleDoorSpawns` (`|MakeArray` (`self.DoorLocation1`) (`self.DoorLocation2`) (`self.DoorLocation3`) (`self.DoorLocation4`) (`self.DoorLocation5`) (`self.DoorLocation6`) (`self.DoorLocation7`) (`self.DoorLocation8`) (`self.DoorLocation9`) (`self.DoorLocation10`)))
  (`parent.UserConstructionScript`))