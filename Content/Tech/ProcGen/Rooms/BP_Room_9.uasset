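; BP_Room_9 is a procedural generation room variant that supplies its own spawn and teleport points to a parent room Blueprint.
; The construction script fills TestedDoorSpawns and ArrowPositions with the same four MovementLocation references, then calls the parent construction script.
; The arrays are set before that parent call, and the event graph holds only disabled default events.
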(fn `UserConstructionScript`
  (bind _array (`|MakeArray` (`self.MovementLocation1`) (`self.MovementLocation2`) (`self.MovementLocation3`) (`self.MovementLocation4`)))
  ;[1 1 1] Set array of possible Spawn and Teleport spawnpoints
  (set `self.TestedDoorSpawns` _array)
  (set `self.ArrowPositions` _array)
  (`parent.UserConstructionScript`))