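; Weapon upgrade component that turns a projectile weapon's shot into two parallel projectiles.
; On BeginPlay it has its owner destroy any other BPC_SingleAttack components in the same slot, so it replaces that attack.
; When fired, it calculates one trajectory and spawns two projectiles offset either side along the player's projectile spawn right vector, passing damage and shot upgrades to both.
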(event `self.ReceiveBeginPlay`
  (for _array_element (`Actor.K2_GetComponentsByClass` (`self.GetOwner`) "/Game/Tech/Upgrades/BPC_SingleAttack.BPC_SingleAttack_C")
    (if (and (!= self _array_element) (== (`/Game/Tech/Upgrades/BPC_BaseUpgrade.Slot` _array_element) (`self.Slot`)))
      (message `/Game/Tech/Upgrades/BPI_UpgradeComponents.I_DestroyComponent` (`self.GetOwner`) _array_element))))

(event `self.Upgrade_ProjectileWeapon`
  (params (`Inaccuracy (half-degrees)` :type "Float (double-precision)") (`Projectile Type` :type "/Game/Tech/Projectiles/BP_BaseProjectile Class Reference") (Damage :type "Float (double-precision)") (`Shot Upgrades` :type "Array of /Game/Tech/Upgrades/BPC_ChainLightning Object Reference (by ref)"))
  (bind (_trajectory_location _trajectory_rotation _trajectory_scale) (`KismetMathLibrary.BreakTransform` (`self.Trajectory`)))
  (set `self.LocationOffset` 20.0)
  (set `self.Trajectory` (`self.F_Calculate Trajectory` `Inaccuracy (half-degrees)`))
  (for _ (range 1 3)
    (`|SpawnActorFromClass` `Projectile Type` (`KismetMathLibrary.MakeTransform` (+ _trajectory_location (* (`SceneComponent.GetRightVector` (`/Game/Tech/Character/BP_Player.Projectilespawn` (cast `/Game/Tech/Character/BP_Player` (`Actor.GetOwner` (`self.GetOwner`)) :!pure true))) (`self.LocationOffset`))) _trajectory_rotation _trajectory_scale) "Undefined" "OverrideRootScale" (`self.GetOwner`) Damage `Shot Upgrades` null)
    (set `self.LocationOffset` (* (`self.LocationOffset`) -1.0))))