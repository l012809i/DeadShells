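; Chain lightning upgrade component that spreads damage between nearby pawns when UpgradeOther is triggered.
; It starts at its owning actor's location, sphere-traces for pawns, then line-traces to each and applies damage via an interface message.
; Each successful hit becomes the next origin, joins the ignore list and recursively calls UpgradeOther, with no explicit jump limit.
; The top-level owner is ignored and credited as instigator; both traces draw debug shapes.
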(event `self.ReceiveBeginPlay`
  (bind _output_get (set `self.Owner` (`Actor.GetOwner` (`Actor.GetOwner` (`self.GetOwner`)))))
  (`KismetArrayLibrary.Array_Add` (`self.Actors to Ignore`) _output_get))

(event `self.Upgrade_Other`
  (bind _location (`self.Location`))
  (`|ExecutionSequence`
    (:`then_0`
      (`/Engine/EditorBlueprintResources/StandardMacros.DoOnce` false
        (:`Completed`
          (set `self.Location` (`Actor.K2_GetActorLocation` (`self.GetOwner`))))))
    (:`then_1`
      (bind _outhits (`KismetSystemLibrary.SphereTraceMultiForObjects` _location _location 200.0 (`|MakeArray` "ObjectTypeQuery3" :!type "EObjectTypeQuery Enum") false (`self.Actors to Ignore`) "ForDuration"))
      (for _array_element _outhits
        (bind (_bblockinghit _binitialoverlap _time _distance _location_2 _impactpoint _normal _impactnormal _physmat _hitactor _hitcomponent _hitbonename _bonename _hititem _elementindex _faceindex _tracestart) (`GameplayStatics.BreakHitResult` _array_element))
        (bind _outhit (`KismetSystemLibrary.LineTraceSingle` _tracestart (`Actor.K2_GetActorLocation` _hitactor) "TraceTypeQuery1" false (`self.Actors to Ignore`) "ForDuration"))
        (bind (_bblockinghit_2 _binitialoverlap_2 _time_2 _distance_2 _location_3 _impactpoint_2 _normal_2 _impactnormal_2 _physmat_2 _hitactor_2) (`GameplayStatics.BreakHitResult` _outhit))
        (bind _target_hit_ (message `/Game/Tech/HealthSystem/BPI_DamageHandling.I_ApplyDamage` _hitactor_2 5.0 (`self.Owner`)))
        (if _target_hit_
          (set `self.Location` (`Actor.K2_GetActorLocation` _hitactor_2))
          (`KismetArrayLibrary.Array_Add` (`self.Actors to Ignore`) _hitactor_2)
          (`self.Upgrade_Other`))))))