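; BPC_BaseUpgrade is a base component for upgrades, each assigned to a Slot on its owning actor.
; On BeginPlay it finds other components of its own class with the same Slot and asks the owner to destroy them through an IDestroyComponent message.
; It declares empty hook events for projectile weapon, melee weapon, hit, player and weapon stat upgrades.
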(event `self.ReceiveBeginPlay`
  (for _array_element (`Actor.K2_GetComponentsByClass` (`self.GetOwner`) (`GameplayStatics.GetObjectClass` self))
    (if (and (!= self _array_element) (== (`/Game/Tech/Upgrades/BPC_BaseUpgrade.Slot` _array_element) (`self.Slot`)))
      (message `/Game/Tech/Upgrades/BPI_UpgradeComponents.I_DestroyComponent` (`self.GetOwner`) _array_element))))

(event `Upgrade_ProjectileWeapon`
  (params (`Inaccuracy (half-degrees)` :type "Float (double-precision)") (`Projectile Type` :type "/Game/Tech/Projectiles/BP_BaseProjectile Class Reference") (Damage :type "Float (double-precision)") (`Shot Upgrades` :type "Array of /Game/Tech/Upgrades/BPC_ChainLightning Object Reference")))

(event `Upgrade_MeleeWeapon`)

(event `Upgrade_Hit`
  (params (Damage :type "Float (double-precision)")))

(event `Upgrade_Player`)

(event `Upgrade_WeaponStat`)