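; Weapon upgrade component that fires three projectiles in a fan from the player's projectile spawn.
; BeginPlay destroys any other BPC_SingleAttack components on the owning weapon, so this attack replaces them.
; UpgradeProjectile calculates one inaccuracy-adjusted trajectory and spawns the projectiles from it, each taking the weapon's damage.
; A DoOnce and FlipFlop switch the sideways and yaw offsets between shots to give right, left and centre projectiles.
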(event `self.ReceiveBeginPlay`
  (for _array_element (`Actor.K2_GetComponentsByClass` (`self.GetOwner`) "/Game/Tech/Upgrades/BPC_SingleAttack.BPC_SingleAttack_C")
    (if (!= self _array_element)
      (message `/Game/Tech/Upgrades/BPI_DestroyComponent.I_DestroyComponent` (`self.GetOwner`) _array_element)
      (`KismetSystemLibrary.PrintString` "del"))))

(event `/Game/Tech/Upgrades/BPC_BaseUpgrade.Upgrade_Projectile`
  (params (`Inaccuracy (half-degrees)` :type "Float (double-precision)") (`Projectile Type` :type "Actor Class Reference"))
  (bind _returnvalue (`self.GetOwner`))
  (bind _trajectory (`self.Trajectory`))
  (set `self.Location Offset` 75.0)
  (set `self.Direction Offset` 15.0)
  (set `self.Trajectory` (`self.F_Calculate Trajectory` `Inaccuracy (half-degrees)`))
  (for _ (range 1 4)
    (bind _returnvalue_2 (`|SpawnActorFromClass` "/Game/Tech/Projectiles/BP_Projectile.BP_Projectile_C" (`KismetMathLibrary.MakeTransform` (+ (* (`self.Location Offset`) (`SceneComponent.GetRightVector` (`/Game/Tech/Character/BP_Player.Projectilespawn` (cast `/Game/Tech/Character/BP_Player` (`Actor.GetOwner` (`self.GetOwner`)) :!pure true)))) (.location _trajectory)) (`KismetMathLibrary.MakeRotator` (.roll (.rotation _trajectory)) (.pitch (.rotation _trajectory)) (+ (.yaw (.rotation _trajectory)) (`self.Direction Offset`))) (.scale _trajectory)) "Undefined" "OverrideRootScale" _returnvalue null))
    (`/Game/Tech/Projectiles/BP_Projectile.Set Damage` _returnvalue_2 (`/Game/Tech/Weapons/WeaponInfo/BP_BaseWeapon.F_GetDamage` (cast `/Game/Tech/Weapons/WeaponInfo/BP_BaseWeapon` _returnvalue :!pure true)))
    (`/Engine/EditorBlueprintResources/StandardMacros.DoOnce` false :!label _label
      (:`Completed`
        (`/Engine/EditorBlueprintResources/StandardMacros.FlipFlop`
          (:`A`
            (set `self.Location Offset` (* (`self.Location Offset`) -1.0))
            (set `self.Direction Offset` (* (`self.Direction Offset`) -1.0))
            (`self.Reset`))
          (:`B`
            (set `self.Location Offset` 0.0)
            (set `self.Direction Offset` 0.0))))))
  (`self.Reset`))

(event `Reset`
  (goto _label :!via `Reset`))