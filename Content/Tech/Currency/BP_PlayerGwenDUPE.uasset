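; Player character blueprint that tracks currency, fires BP_Projectile and relays health changes to the UI.
; Damage and healing interface calls forward to BPCHealthComponent; they, currency changes and a tick-delayed BeginPlay fire UI update dispatchers.
; Look axes rotate the mesh from a single axis value past a deadzone, while LookAtMouse is defined but never called here.
; Only Right-axis movement is wired, and keys 3/4 test damage and healing.
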(event `/Game/Tech/Currency/BPI_Currency.Collect`
  (params (AmountCollected :type "Float (double-precision)"))
  ;[0.9922 0.6353 1] Currency events
  (set `self.Current currency` (+ (`self.Current currency`) AmountCollected))
  (`self.E_CurrencyUpdated` :!label _label))

(event `InputAction|PrimaryWeaponfire`
  (params (Key :type "Key Structure"))
  ;[0.9922 0.6353 1] Spawns projectile on left click at location of arrow
  (:`Pressed`
    (`|SpawnActorFromClass` "/Game/Tech/Projectiles/BP_Projectile.BP_Projectile_C" (`SceneComponent.K2_GetComponentToWorld` (`self.Projectilespawn`)) "Undefined" "OverrideRootScale" self null)))

(event `self.ReceiveBeginPlay`
  ;[0 1 1] BeginPlay - Call UI event dispatcher to update values
  (`KismetSystemLibrary.DelayUntilNextTick`)
  (`self.E_HealthUpdated` (`/Game/Tech/HealthSystem/BPC_HealthComponent.S_Health` (`self.BPC_HealthComponent`)))
  (`self.E_CurrencyUpdated`))

(event `/Game/Tech/Currency/BPI_Currency.RemoveCurrency`
  (params (AmountRemoved :type "Float (double-precision)"))
  ;[0.9922 0.6353 1] Currency events
  (set `self.Current currency` (- (`self.Current currency`) AmountRemoved))
  (goto _label))

(event `Key|Three`
  (params (Key :type "Key Structure"))
  ;[0 0.5 1] Debug - Testing I_Apply_Damage
  (:`Pressed`
    (`self.I_ApplyDamage` 3.0 self)))

(event `InputAxis|look up`
  (params (AxisValue :type "Float (single-precision)"))
  (bind _returnvalue (`KismetMathLibrary.MakeVector` (stale `InputAxis|Look right` AxisValue) AxisValue))
  (if (> (`KismetMathLibrary.VSize` _returnvalue) 0.25) :!label _label_2
    (`SceneComponent.K2_SetWorldRotation` (`self.Mesh`) (`KismetMathLibrary.Conv_VectorToRotator` _returnvalue) false false)))

(event `InputAxis|Look right`
  (params (AxisValue :type "Float (single-precision)"))
  (goto _label_2))

(event `Key|Four`
  (params (Key :type "Key Structure"))
  ;[0 0.5 1] Debug - Testing I_Apply_Healing
  (:`Pressed`
    (`self.I_ApplyHealing` 3.0 self)))

(event `InputAxis|Forward`
  (params (AxisValue :type "Float (single-precision)")))

(event `InputAxis|Right`
  (params (AxisValue :type "Float (single-precision)"))
  (`self.AddMovementInput` (0.0 1.0 0.0) AxisValue))

(fn `I_ApplyDamage`
  (params (Amount :type "Float (double-precision)") (Instigator :type "Actor Object Reference"))
  (returns (`Target Dead?` :type Boolean))
  (bind _bpc_healthcomponent (`self.BPC_HealthComponent`))
  ;[0 1 1] Sending damage to health component and updating event dispatcher for UI
  (bind _target_dead_ (`/Game/Tech/HealthSystem/BPC_HealthComponent.I_ApplyDamage` _bpc_healthcomponent Amount Instigator))
  (`self.E_HealthUpdated` (`/Game/Tech/HealthSystem/BPC_HealthComponent.S_Health` _bpc_healthcomponent))
  (return _target_dead_))

(fn `I_ApplyHealing`
  (params (Amount :type "Float (double-precision)") (Instigator :type "Actor Object Reference"))
  (returns (`Target Full?` :type Boolean))
  (bind _bpc_healthcomponent (`self.BPC_HealthComponent`))
  ;[0 1 1] Sending healing to health component and updating event dispatcher for UI
  (bind _target_full_ (`/Game/Tech/HealthSystem/BPC_HealthComponent.I_ApplyHealing` _bpc_healthcomponent Amount Instigator))
  (`self.E_HealthUpdated` (`/Game/Tech/HealthSystem/BPC_HealthComponent.S_Health` _bpc_healthcomponent))
  (return _target_full_))

(fn `Look at mouse`
  (bind (_returnvalue_roll _returnvalue_pitch _returnvalue_yaw) (`KismetMathLibrary.BreakRotator` (`KismetMathLibrary.FindLookAtRotation` (`self.K2_GetActorLocation` self) (`.Location` (`GameplayStatics.BreakHitResult` (`PlayerController.GetHitResultUnderCursorByChannel` (`GameplayStatics.GetPlayerController` 0) "TraceTypeQuery1" true))))))
  (`SceneComponent.K2_SetWorldRotation` (`self.Mesh`) (`KismetMathLibrary.MakeRotator` 0.0 0.0 (- _returnvalue_yaw 90.0)) false false))

(fn `UserConstructionScript`)