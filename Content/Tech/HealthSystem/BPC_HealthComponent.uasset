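; Health component that tracks its owner's health in an S_Health struct and serves damage, healing, max health and struct queries through interface functions.
; Damage and healing clamp health between zero and max, returning whether the target is dead or fully healed.
; Lowering max health trims current health to prevent overheal.
; Debug subgraphs print instigator, target and value details, but no UI dispatcher calls appear despite comments mentioning them.
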(fn `I_ApplyDamage`
  (params (Damage :type "Float (double-precision)") (Instigator :type "Actor Object Reference"))
  (returns (`Target Hit?` :type Boolean) (`Target Dead?` :type Boolean))
  (bind (_health _maxhealth) (break `/Game/Tech/HealthSystem/S_Health` (`self.S_Health`)))
  ;[0 1 1] Subtract damage from health using S_Health structure
  (`KismetSystemLibrary.PrintText` (`|FormatText` (`KismetSystemLibrary.GetDisplayName` (`self.GetOwner`)) "Instigated By: {target} \nTarget: {self} \nDamage: {amount} \nOld Health: {health}" (`KismetSystemLibrary.GetDisplayName` Instigator) Damage _health) true true (struct :`R` 0.5 :`A` 1.0) 3.0)
  (bind _structout (setmembers `/Game/Tech/HealthSystem/S_Health` :`StructRef` (`self.S_Health`) :`Health` (`KismetMathLibrary.FClamp` (- _health (`local.Damage`)) 0.0 _maxhealth)))
  (bind _health_2 (break `/Game/Tech/HealthSystem/S_Health` _structout))
  (bind _returnvalue (<= _health_2 0.0))
  ;[0 1 1] Call event dispatcher for UI and check if player is dead
  (`KismetSystemLibrary.PrintText` (`|FormatText` "New Health: {amount} \nTarget Dead: {bool}" _health_2 _returnvalue) true true (struct :`R` 0.5 :`A` 1.0) 3.0)
  (return true _returnvalue))

(fn `I_ApplyHealing`
  (params (Healing :type "Float (double-precision)") (Instigator :type "Actor Object Reference"))
  (returns (`Target Full?` :type Boolean))
  (bind (_health _maxhealth) (break `/Game/Tech/HealthSystem/S_Health` (`self.S_Health`)))
  ;[0 1 1] Add healing to health using S_Health structure
  (`KismetSystemLibrary.PrintText` (`|FormatText` (`KismetSystemLibrary.GetDisplayName` (`self.GetOwner`)) "Instigated By:  {instigator} \nTarget: {self} \nHealing: {amount} \nOld Health: {health}" (`KismetSystemLibrary.GetDisplayName` Instigator) Healing _health) true true (struct :`G` 0.5 :`A` 1.0) 3.0)
  (bind _structout (setmembers `/Game/Tech/HealthSystem/S_Health` :`StructRef` (`self.S_Health`) :`Health` (`KismetMathLibrary.FClamp` (+ _health (`local.Healing`)) 0.0 _maxhealth)))
  (bind (_health_2 _maxhealth_2) (break `/Game/Tech/HealthSystem/S_Health` _structout))
  (bind _returnvalue (>= _health_2 _maxhealth_2))
  ;[0 1 1] Call event dispatcher for UI and check if player is full hp
  (`KismetSystemLibrary.PrintText` (`|FormatText` "New Health: {amount} \nTarget Full: {bool}" _health_2 _returnvalue) true true (struct :`G` 0.5 :`A` 1.0) 3.0)
  (return _returnvalue))

(fn `I_ChangeMaxHealth`
  (params (`Max Health` :type "Float (double-precision)") (Instigator :type "Actor Object Reference"))
  (returns (`Return Value` :type Boolean))
  (bind _s_health (`self.S_Health`))
  ;[0 1 1] Get the target max health and set the max health making sure overhealing doesn't occur
  (bind _structout (setmembers `/Game/Tech/HealthSystem/S_Health` :`StructRef` (`self.S_Health`) :`Max Health` `Max Health`))
  (bind (_health _maxhealth) (break `/Game/Tech/HealthSystem/S_Health` _structout))
  (bind _returnvalue (> _health _maxhealth))
  (if _returnvalue
    (setmembers `/Game/Tech/HealthSystem/S_Health` :`StructRef` _s_health :`Health` (`.MaxHealth_5_66D911EB4E67FC9A695B02A3D74B2773` (break `/Game/Tech/HealthSystem/S_Health` _s_health))))
  (`KismetSystemLibrary.PrintText` (`|FormatText` "Old Max Health: {old} \nNew Max Health: {new} \nSet Health: {bool}" (`local.Max Health`) (`.MaxHealth_5_66D911EB4E67FC9A695B02A3D74B2773` (break `/Game/Tech/HealthSystem/S_Health` (`self.S_Health`))) _returnvalue))
  (return _returnvalue))

(fn `I_GetHealthStruct`
  (returns (`Health Struct` :type "/Game/Tech/HealthSystem/S_Health Structure"))
  ;[0 1 1] Pass through health struct
  (return (`self.S_Health`)))