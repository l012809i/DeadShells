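; BP_NormalProjectile is a projectile that deals damage to whatever its sphere collider hits, then destroys itself.
; On hit it sends the damage through an interface message to the other actor, with its owner as instigator.
; If that call reports a target hit, every BPC_BaseUpgrade component on the projectile is notified with the damage, so upgrades act as modular on-hit effects.
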(event `self.Sphere_Col.OnComponentHit`
  (params (HitComponent :type "PrimitiveComponent Object Reference") (OtherActor :type "Actor Object Reference") (OtherComp :type "PrimitiveComponent Object Reference") (NormalImpulse :type "Vector Structure") (Hit :type "HitResult Structure (by ref)"))
  (bind _target_hit_ (message `/Game/Tech/HealthSystem/BPI_DamageHandling.I_ApplyDamage` OtherActor (`self.Damage`) (`self.GetOwner`)))
  (if _target_hit_
    (for _array_element (`self.K2_GetComponentsByClass` "/Game/Tech/Upgrades/BPC_BaseUpgrade.BPC_BaseUpgrade_C")
      (`/Game/Tech/Upgrades/BPC_BaseUpgrade.Upgrade_Hit` _array_element (`self.Damage`))))
  (`self.K2_DestroyActor`))

(fn `UserConstructionScript`
  (`parent.UserConstructionScript`))