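; BP_Projectile is a projectile actor that damages what it overlaps and destroys itself on impact.
; Its damage is set through the SetDamage event and sent on sphere overlap via the IApplyDamageMessage interface, with its owner as instigator.
; When that call reports a target hit, it calls UpgradeOther on each of its BPC_BaseUpgrade components before destroying itself.
; A blocking hit on the sphere destroys it without applying damage, and both collision paths print debug text.
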(event `Set Damage`
  (params (Damage :type "Float (double-precision)"))
  (set `self.Damage` Damage))

(event `self.Sphere_Col.OnComponentBeginOverlap`
  (params (OverlappedComponent :type "PrimitiveComponent Object Reference") (OtherActor :type "Actor Object Reference") (OtherComp :type "PrimitiveComponent Object Reference") (OtherBodyIndex :type Integer) (bFromSweep :type Boolean) (SweepResult :type "HitResult Structure (by ref)"))
  ;[1 1 1] Applying Damage to the enemy and destroys on impact
  (bind _target_hit_ (message `/Game/Tech/HealthSystem/BPI_DamageHandling.I_ApplyDamage` OtherActor (`self.Damage`) (`self.GetOwner`)))
  (`KismetSystemLibrary.PrintString` (`KismetStringLibrary.Conv_BoolToString` _target_hit_))
  (if _target_hit_
    (for _array_element (`self.K2_GetComponentsByClass` "/Game/Tech/Upgrades/BPC_BaseUpgrade.BPC_BaseUpgrade_C")
      (`/Game/Tech/Upgrades/BPC_BaseUpgrade.Upgrade_Other` _array_element))
    (`self.K2_DestroyActor`)))

(event `self.Sphere_Col.OnComponentHit`
  (params (HitComponent :type "PrimitiveComponent Object Reference") (OtherActor :type "Actor Object Reference") (OtherComp :type "PrimitiveComponent Object Reference") (NormalImpulse :type "Vector Structure") (Hit :type "HitResult Structure (by ref)"))
  ;[1 1 1] Projectile destroys on object hit
  (`KismetSystemLibrary.PrintString` "Object Hit!" true true (struct :`G` 1.0 :`B` 0.048421 :`A` 1.0))
  (`self.K2_DestroyActor`))

(fn `UserConstructionScript`)