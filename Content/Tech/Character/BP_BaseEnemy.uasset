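; BP_BaseEnemy is a base enemy Blueprint that can take damage and receive healing through interface functions.
; Both functions forward the amount and instigator to a health component and return that component's result.
; After each call, it fires a health-updated event dispatcher with the component's health value so the UI can refresh.
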(fn `I_ApplyDamage`
  (params (Amount :type "Float (double-precision)") (Instigator :type "Actor Object Reference"))
  (returns (`Target Dead?` :type Boolean))
  (bind _bpc_healthcomponent (`self.BPC_HealthComponent`))
  ;[0 1 1] Sending damage to health component and updating event dispatcher for UI
  (bind _target_dead_ (`/Game/Tech/HealthSystem/BPC_HealthComponent.I_ApplyDamage` _bpc_healthcomponent Amount Instigator))
  (`self.E_HealthUpdated` (`/Game/Tech/HealthSystem/BPC_HealthComponent.S_Health` _bpc_healthcomponent))
  (return _target_dead_))

(fn `I_ApplyHealing`
  (params (Amount :type "Float (double-precision)") (Instigator :type "Actor Object Reference"))
  (returns (`Target Full?` :type Boolean))
  (bind _bpc_healthcomponent (`self.BPC_HealthComponent`))
  ;[0 1 1] Sending healing to health component and updating event dispatcher for UI
  (bind _target_full_ (`/Game/Tech/HealthSystem/BPC_HealthComponent.I_ApplyHealing` _bpc_healthcomponent Amount Instigator))
  (`self.E_HealthUpdated` (`/Game/Tech/HealthSystem/BPC_HealthComponent.S_Health` _bpc_healthcomponent))
  (return _target_full_))

(fn `UserConstructionScript`)