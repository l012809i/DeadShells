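; Base melee grunt enemy that takes damage and healing through interface functions and dies as a ragdoll.
; BPCHealthComponent processes both, then a health-updated dispatcher fires for UI; lethal damage enables mesh physics and a timer later destroys the actor.
; A looping timer started at BeginPlay draws current health above the mesh as debug text.
; Random roaming via AI MoveTo is present but unconnected, so it never runs.
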(event `self.ReceiveBeginPlay`
  (`self.Display Debug Health`))

(event `Random Roam`
  ;[1 1 1] AI Roaming - Roaming to itself (creating random location)
)

(event `Display Debug Health`
  ;[1 1 1] Debug Health Temp - Displays health above enemies head for debugging purposes
  (`KismetSystemLibrary.K2_SetTimerDelegate` (delegate `DebugHealth`) 0.01 true) ; Better than Delay
)

(event `DebugHealth`
  ;[1 1 1] Debug Health Temp - Displays health above enemies head for debugging purposes
  (`KismetSystemLibrary.DrawDebugString` (`KismetMathLibrary.MakeVector` (.x (`SceneComponent.K2_GetComponentLocation` (`self.Mesh`))) (- (.y (`SceneComponent.K2_GetComponentLocation` (`self.Mesh`))) 35.0) (+ (.z (`SceneComponent.K2_GetComponentLocation` (`self.Mesh`))) 220.0)) (`KismetStringLibrary.Conv_DoubleToString` (`.Health_4_D29B34A6447D561A7C4BF3AD8D470278` (break `/Game/Tech/HealthSystem/S_Health` (`/Game/Tech/HealthSystem/BPC_HealthComponent.S_Health` (`self.BPC_HealthComponent`))))) null (struct :`R` 1.0 :`B` 0.014804 :`A` 1.0)))

(fn `Death`
  (`self.K2_DestroyActor`))

(fn `I Get BP Base Enemy`
  (returns (Enemy :type "Character Object Reference"))
  (return self))

(fn `I_ApplyDamage`
  (params (Damage :type "Float (double-precision)") (Instigator :type "Actor Object Reference"))
  (returns (`Target Dead?` :type Boolean))
  (bind _bpc_healthcomponent (`self.BPC_HealthComponent`))
  ;[0 1 1] Sending damage to health component and updating event dispatcher for UI
  (bind _target_dead_ (`/Game/Tech/HealthSystem/BPC_HealthComponent.I_ApplyDamage` _bpc_healthcomponent Damage Instigator))
  (`self.E_HealthUpdated` (`/Game/Tech/HealthSystem/BPC_HealthComponent.S_Health` _bpc_healthcomponent))
  (if _target_dead_
    (`PrimitiveComponent.SetSimulatePhysics` (`self.Mesh`) true) ; Enable Ragdoll
    (bind _returnvalue (`KismetSystemLibrary.K2_SetTimer` null "Death" 5.0)) ; 5 Second delay before Destroying Character
    (set `self.TimerHandler` _returnvalue)
    (return _target_dead_)
    (else
      (return false))))

(fn `I_ApplyHealing`
  (params (Healing :type "Float (double-precision)") (Instigator :type "Actor Object Reference"))
  (returns (`Target Full?` :type Boolean))
  (bind _bpc_healthcomponent (`self.BPC_HealthComponent`))
  ;[0 1 1] Sending healing to health component and updating event dispatcher for UI
  (bind _target_full_ (`/Game/Tech/HealthSystem/BPC_HealthComponent.I_ApplyHealing` _bpc_healthcomponent Healing Instigator))
  (`self.E_HealthUpdated` (`/Game/Tech/HealthSystem/BPC_HealthComponent.S_Health` _bpc_healthcomponent))
  (return _target_full_))

(fn `UserConstructionScript`)