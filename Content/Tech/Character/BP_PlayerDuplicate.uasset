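; Top-down player character handling movement, eight-way dodge launches, cursor-facing aim, interaction, weapons, currency and health.
; Weapon pickups reject duplicates and fill a slot inventory, dropping a pickup when full; switching toggles visibility of socket-attached weapons.
; Upgrade components apply to the player and their slot's weapon, while health interface calls forward to a health component and notify UI through dispatchers.
; Hub world skips cursor facing and starts with a timed physics-mesh reattach.
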(event `/Game/Tech/Pickups/BPI_CharacterInteract.WeaponUIInteract`
  (params (WeaponName :type "/Game/Tech/Weapons/E_WeaponNames Enum" :default "NewEnumerator4") (WeaponPickup :type "Actor Object Reference") (WeaponDescription :type String))
  (bind _weapon_pickup (`self.Weapon Pickup`))
  (bind _weapon_inventory (`self.Weapon_Inventory`))
  ;[0.9922 0.6353 1] Bypasses the UI if the player has not got a weapon or only has one weapon
  (set `self.Weapon Pickup` WeaponPickup)
  (set `self.DuplicateWeapon` false)
  (if (`KismetArrayLibrary.Array_IsEmpty` _weapon_inventory)
    (message `/Game/Tech/Pickups/BPI_CharacterInteract.Addweapon` _weapon_pickup 0)
    (elif (== (`KismetArrayLibrary.Array_LastIndex` _weapon_inventory) 0)
      (message `/Game/Tech/Pickups/BPI_CharacterInteract.Addweapon` _weapon_pickup 1)
      (else
        ;[0.9922 0.6353 1] Stops player from picking up duplicate weapon
        (for _array_element (`self.Weapon_Inventory`)
          (bind _returnvalue (`|EnumEquality` (`.WeaponName_34_C3694ECA427C22994D707E9D808D1F6C` (break `/Game/Tech/Weapons/WeaponInfo/WeaponInformation` (`/Game/Tech/Weapons/WeaponInfo/BP_BaseWeapon.WeaponInformation` _array_element))) WeaponName))
          (if _returnvalue
            (set `self.DuplicateWeapon` true)
            (elif (`self.DuplicateWeapon`)
              (set `self.DuplicateWeapon` true)
              (elif _returnvalue
                (set `self.DuplicateWeapon` true)
                (else
                  (set `self.DuplicateWeapon` false))))))
        (if (`self.DuplicateWeapon`)
          (`KismetSystemLibrary.PrintString` "Duplicate weapon")
          (else
            (`self.WeaponUIUpdate` WeaponPickup WeaponDescription)))))))

(event `Restore Mesh`
  (`PrimitiveComponent.SetSimulatePhysics` (`self.Mesh`) true)
  (`SceneComponent.K2_AttachToComponent` (`self.Mesh`) (`self.CapsuleComponent`) "None" "KeepRelative" "KeepRelative" "KeepRelative" true)
  (`SceneComponent.K2_SetRelativeLocationAndRotation` (`self.Mesh`) (-10.0 0.0 -60.0) (struct :`Yaw` -90.0) false false))

(event `InputAction|Interact`
  (params (Key :type "Key Structure"))
  (bind _projectilespawn (`self.Projectilespawn`))
  (bind _returnvalue (`SceneComponent.K2_GetComponentLocation` _projectilespawn))
  ;[0.9922 0.6353 1] Line Trace for pickups
  (:`Pressed`
    (bind _outhit (`KismetSystemLibrary.LineTraceSingleForObjects` :`Start` _returnvalue :`End` (+ _returnvalue (* (`SceneComponent.GetForwardVector` _projectilespawn) 2.0)) :`ObjectTypes` (`|MakeArray` "ObjectTypeQuery2" :!type "EObjectTypeQuery Enum") :`DrawDebugType` "ForDuration"))
    (message `/Game/Tech/Pickups/BPI_CharacterInteract.Interact` (`.HitActor` (`GameplayStatics.BreakHitResult` _outhit)) self)))

(event `self.ReceiveBeginPlay`
  (if (`self.InHubWorld?`)
    (`PrimitiveComponent.SetSimulatePhysics` (`self.Mesh`) true)
    (`KismetSystemLibrary.K2_SetTimerDelegate` (delegate `Restore Mesh`) 2.0)
    (else
      ;[0 1 1] BeginPlay - Call UI event dispatcher to update values
      (`KismetSystemLibrary.DelayUntilNextTick`)
      (`self.E_HealthUpdated` (`/Game/Tech/HealthSystem/BPC_HealthComponent.S_Health` (`self.BPC_HealthComponent`)))
      (`self.E_CurrencyUpdated`)
      ;[0 0.5 1] Debug - adding upgrade components
      (for _array_element (`|MakeArray` null :!type "/Game/Tech/Upgrades/BPC_BaseUpgrade Class Reference")
        (`self.I_InitialiseComponent` _array_element))
      (for _array_element_2 (`|MakeArray` null :!type "/Game/Tech/Upgrades/BPC_BaseUpgrade Class Reference")
        (`self.I_InitialiseComponent` _array_element_2 1)))))

(event `InputAction|Interact`
  (params (Key :type "Key Structure"))
  (:`Pressed`
    (for _array_element (`self.GetOverlappingActors` null)
      (if (`KismetSystemLibrary.DoesImplementInterface` _array_element "/Game/Tech/HubWorld/BPI_Interact.BPI_Interact_C")
        (`/Engine/EditorBlueprintResources/StandardMacros.FlipFlop`
          (:`A`
            (message `/Game/Tech/HubWorld/BPI_Interact.Interact` _array_element)
            (set `self.CanMove?` false)
            (break))
          (:`B`
            (message `/Game/Tech/HubWorld/BPI_Interact.Interact` _array_element)
            (set `self.CanMove?` true)
            (break)))))))

(event `/Game/Tech/Currency/BPI_Currency.Collect`
  (params (AmountCollected :type "Float (double-precision)"))
  ;[0.9922 0.6353 1] Add and Remove Currency
  (set `self.Current currency` (+ (`self.Current currency`) AmountCollected))
  (`self.E_CurrencyUpdated` :!label _label))

(event `/Game/Tech/Currency/BPI_Currency.RemoveCurrency`
  (params (AmountRemoved :type "Float (double-precision)"))
  ;[0.9922 0.6353 1] Add and Remove Currency
  (set `self.Current currency` (- (`self.Current currency`) AmountRemoved))
  (goto _label))

(event `self.ReceiveTick`
  (params (DeltaSeconds :type "Float (single-precision)"))
  ;[0 1 0.05286] Used For Mouse Direction And Rotate Character To That Direction
  (`self.Look At Cursor`))

(event `Key|Three`
  (params (Key :type "Key Structure"))
  ;[0 0.5 1] Debug - Testing I_Apply_Damage
  (:`Pressed`
    (`self.I_ApplyDamage` 3.0 self)))

(event `InputAxis|MoveForward`
  (params (AxisValue :type "Float (single-precision)"))
  ;[0 1 0.05286] Character Movement
  (if (`self.CanMove?`)
    (`self.AddMovementInput` (`KismetMathLibrary.GetForwardVector` (`self.GetControlRotation`)) AxisValue)
    (if (== AxisValue 0.0)
      (set `self.PlayerMoving?` false)
      (else
        (set `self.PlayerMoving?` true)))))

(event `InputAction|dodge`
  (params (Key :type "Key Structure"))
  (:`Pressed`
    (`|ExecutionSequence`
      (:`then_0`
        (if (`self.Dodge Up`)
          (`self.LaunchCharacter` (`self.dodge direction`) true :!label _label_2)
          (`GameplayStatics.PlaySound2D` "/Game/Tech/Sounds/PlayerSounds/Dash/Player_Dash_Fixed.Player_Dash_Fixed" 1.0 1.0 0.0 null null)))
      (:`then_1`
        (if (`self.Dodge Down`)
          (goto _label_2)))
      (:`then_2`
        (if (`self.Dodge Left`)
          (goto _label_2)))
      (:`then_3`
        (if (`self.Dodge Right`)
          (goto _label_2)))
      (:`then_4`
        (if (`self.Dodge Up/Left`)
          (goto _label_2)))
      (:`then_5`
        (if (`self.Dodge Down/Left`)
          (goto _label_2)))
      (:`then_6`
        (if (`self.Dodge Up/Right`)
          (goto _label_2)))
      (:`then_7`
        (if (`self.Dodge Down/Right`)
          (goto _label_2))))))

(event `Key|Four`
  (params (Key :type "Key Structure"))
  ;[0 0.5 1] Debug - Testing I_Apply_Healing
  (:`Pressed`
    (`self.I_ApplyHealing` 3.0 self)))

(event `InputAxis|MoveRight`
  (params (AxisValue :type "Float (single-precision)"))
  ;[0 1 0.05286] Character Movement
  (if (`self.CanMove?`)
    (`self.AddMovementInput` (`KismetMathLibrary.GetRightVector` (`self.GetControlRotation`)) AxisValue)
    (if (== AxisValue 0.0)
      (set `self.PlayerMoving?` false)
      (else
        (set `self.PlayerMoving?` true)))))

(event `Key|A`
  (params (Key :type "Key Structure"))
  (:`Pressed`
    (if (`self.Dodge Up`)
      (set `self.Dodge Up/Left` true)
      (set `self.dodge direction` (3000.0 -3000.0 0.0))
      (elif (`self.Dodge Down`)
        (set `self.Dodge Down/Left` false)
        (set `self.dodge direction` (-3000.0 -3000.0 0.0))
        (else
          (set `self.Dodge Up` false)
          (set `self.Dodge Down` false)
          (set `self.Dodge Left` true)
          (set `self.Dodge Right` false)
          (set `self.dodge direction` (0.0 -3000.0 0.0))))))
  (:`Released`
    (set `self.Dodge Left` false)
    (set `self.Dodge Up/Left` false)
    (set `self.Dodge Down/Left` false)))

(event `Key|W`
  (params (Key :type "Key Structure"))
  (:`Pressed`
    (if (`self.Dodge Left`)
      (set `self.Dodge Up/Left` true)
      (set `self.dodge direction` (3000.0 -3000.0 0.0))
      (elif (`self.Dodge Right`)
        (set `self.Dodge Up/Right` true)
        (set `self.dodge direction` (3000.0 3000.0 0.0))
        (else
          (set `self.Dodge Up` true)
          (set `self.Dodge Down` false)
          (set `self.Dodge Left` false)
          (set `self.Dodge Right` false)
          (set `self.dodge direction` (3000.0 0.0 0.0))))))
  (:`Released`
    (set `self.Dodge Up` false)
    (set `self.Dodge Up/Left` false)
    (set `self.Dodge Up/Right` false)))

(event `Key|S`
  (params (Key :type "Key Structure"))
  (:`Pressed`
    (if (`self.Dodge Left`)
      (set `self.Dodge Down/Left` true)
      (set `self.dodge direction` (-3000.0 -3000.0 0.0))
      (elif (`self.Dodge Right`)
        (set `self.Dodge Down/Right` true)
        (set `self.dodge direction` (-3000.0 3000.0 0.0))
        (else
          (set `self.Dodge Up` false)
          (set `self.Dodge Down` true)
          (set `self.Dodge Left` false)
          (set `self.Dodge Right` false)
          (set `self.dodge direction` (-3000.0 0.0 0.0))))))
  (:`Released`
    (set `self.Dodge Down` false)
    (set `self.Dodge Down/Left` false)
    (set `self.Dodge Down/Right` false)))

(event `Key|D`
  (params (Key :type "Key Structure"))
  (:`Pressed`
    (if (`self.Dodge Up`)
      (set `self.Dodge Up/Right` true)
      (set `self.dodge direction` (3000.0 3000.0 0.0))
      (elif (`self.Dodge Down`)
        (set `self.Dodge Down/Right` true)
        (set `self.dodge direction` (-3000.0 3000.0 0.0))
        (else
          (set `self.Dodge Up` false)
          (set `self.Dodge Down` false)
          (set `self.Dodge Left` false)
          (set `self.Dodge Right` true)
          (set `self.dodge direction` (0.0 3000.0 0.0))))))
  (:`Released`
    (set `self.Dodge Right` false)
    (set `self.Dodge Up/Right` false)
    (set `self.Dodge Down/Right` false)))

(event `InputAction|AlternateWeaponFire`
  (params (Key :type "Key Structure"))
  (bind _output (`|GetArrayItem` (`self.Weapon_Inventory`) (`self.WeaponSlot`)))
  ;[0 1 1] Alternate Weapon fire
  (:`Pressed`
    (`/Engine/EditorBlueprintResources/StandardMacros.IsValid` _output
      (:`Is Valid`
        (`/Game/Tech/Weapons/WeaponInfo/BP_BaseWeapon.AlternateActivate` _output))))
  (:`Released`
    (`/Engine/EditorBlueprintResources/StandardMacros.IsValid` _output
      (:`Is Valid`
        (`/Game/Tech/Weapons/WeaponInfo/BP_BaseWeapon.AlternateDeactivate` _output)))))

(event `InputAction|PrimaryWeaponfire`
  (params (Key :type "Key Structure"))
  (bind _output (`|GetArrayItem` (`self.Weapon_Inventory`) (`self.WeaponSlot`)))
  ;[0 1 1] WeaponFire input - activate and deactivate currently equipped weapon
  (:`Pressed`
    (`/Engine/EditorBlueprintResources/StandardMacros.IsValid` _output
      (:`Is Valid`
        (`/Game/Tech/Weapons/WeaponInfo/BP_BaseWeapon.ActivateWeapon` _output))))
  (:`Released`
    (`/Engine/EditorBlueprintResources/StandardMacros.IsValid` _output
      (:`Is Valid`
        (`/Game/Tech/Weapons/WeaponInfo/BP_BaseWeapon.DeactivateWeapon` _output false)))))

(event `SwitchWeapon`
  (bind _output (`|GetArrayItem` (`self.Weapon_Inventory`) (`self.PreviousWeaponSlot`)))
  ;[0 1 1] SwitchWeapon - deactivate the previous weapon, make it invisible and make the new weapon visible
  (if (== (`self.WeaponSlot`) (`self.PreviousWeaponSlot`))
    (`KismetSystemLibrary.PrintText` (`|FormatText` "Weapon not switched") true true (struct :`R` 0.5 :`B` 0.5 :`A` 1.0) 3.0)
    (else
      (`KismetSystemLibrary.PrintText` (`|FormatText` "Switched from {x} : {old} to {y} : {new}" (`self.PreviousWeaponSlot`) (`KismetSystemLibrary.GetClassDisplayName` (`GameplayStatics.GetObjectClass` (`|GetArrayItem` (`self.Weapon_Inventory`) (`self.PreviousWeaponSlot`)))) (`self.WeaponSlot`) (`KismetSystemLibrary.GetClassDisplayName` (`GameplayStatics.GetObjectClass` (`|GetArrayItem` (`self.Weapon_Inventory`) (`self.WeaponSlot`))))) true true (struct :`R` 0.5 :`B` 0.5 :`A` 1.0) 3.0)))
  (if (not (== (`self.WeaponSlot`) (`self.PreviousWeaponSlot`)))
    (`/Engine/EditorBlueprintResources/StandardMacros.IsValid` _output
      (:`Is Valid`
        (`/Game/Tech/Weapons/WeaponInfo/BP_BaseWeapon.DeactivateWeapon` _output true)
        (`SceneComponent.SetVisibility` (`/Game/Tech/Weapons/WeaponInfo/BP_BaseWeapon.DefaultSceneRoot` _output) false true)
        (`SceneComponent.SetVisibility` (`/Game/Tech/Weapons/WeaponInfo/BP_BaseWeapon.DefaultSceneRoot` (`|GetArrayItem` (`self.Weapon_Inventory`) (`self.WeaponSlot`))) true true)))))

(event `InputAction|InventorySlotUp`
  (params (Key :type "Key Structure"))
  ;[0 1 1] Switch Weapon Slot - set the previous and new weapon indexes. Making sure the new index is within the inventory limits
  (:`Pressed`
    (set `self.PreviousWeaponSlot` (`self.WeaponSlot`))
    (`/Engine/EditorBlueprintResources/StandardMacros.IncrementInt` (`self.WeaponSlot`)
      (:`  `
        (if (>= (`self.WeaponSlot`) (`KismetArrayLibrary.Array_Length` (`self.Weapon_Inventory`)))
          (set `self.WeaponSlot` 0))
        (`self.SwitchWeapon`)))))

(event `InputAction|InventorySlotDown`
  (params (Key :type "Key Structure"))
  (bind _returnvalue (`KismetArrayLibrary.Array_Length` (`self.Weapon_Inventory`)))
  ;[0 1 1] Switch Weapon Slot - set the previous and new weapon indexes. Making sure the new index is within the inventory limits
  (:`Pressed`
    (set `self.PreviousWeaponSlot` (`self.WeaponSlot`))
    (bind _result (`/Engine/EditorBlueprintResources/StandardMacros.DecrementInt` (`self.WeaponSlot`))
      (:`  `
        (if (< _result 0)
          (set `self.WeaponSlot` (`KismetMathLibrary.Clamp` (- _returnvalue 1) 0 _returnvalue)))
        (`self.SwitchWeapon`)))))

(event `self.I_AddAndAttachWeapon`
  (params (`Weapon Class` :type "/Game/Tech/Weapons/WeaponInfo/BP_BaseWeapon Class Reference") (`Inventory Index` :type Integer))
  (bind _defaultsceneroot (`/Game/Tech/Weapons/WeaponInfo/BP_BaseWeapon.DefaultSceneRoot` (`self.SpawnedWeapon`)))
  ;[0 1 1] Add and Attach Weapon - Spawn weapon of class, attaching that weapon to the mesh. Then add the weapon in the WeaponInventory array of the selected slot, checking to see if we need to make the new weapon visible
  (bind _returnvalue (`|SpawnActorFromClass` `Weapon Class` (`KismetMathLibrary.MakeTransform` (`self.K2_GetActorLocation`)) "AlwaysSpawn" "OverrideRootScale" self null))
  (bind _output_get (set `self.SpawnedWeapon` _returnvalue))
  (`self.K2_AttachToComponent` _output_get (`self.Mesh`) "WeaponLocation" "SnapToTarget" "SnapToTarget" "SnapToTarget" true)
  (`KismetArrayLibrary.Array_Set` (`self.Weapon_Inventory`) `Inventory Index` (`self.SpawnedWeapon`) true)
  (`KismetSystemLibrary.PrintText` (`|FormatText` "{weapon} added at slot {x}" (`KismetSystemLibrary.GetClassDisplayName` (`GameplayStatics.GetObjectClass` (`self.SpawnedWeapon`))) (`KismetArrayLibrary.Array_Find` (`self.Weapon_Inventory`) (`self.SpawnedWeapon`))) true true (struct :`R` 0.5 :`B` 0.5 :`A` 1.0) 3.0)
  (if (== (`KismetArrayLibrary.Array_Find` (`self.Weapon_Inventory`) (`self.SpawnedWeapon`)) (`self.WeaponSlot`))
    (`SceneComponent.SetVisibility` _defaultsceneroot true true)
    (set `self.isHoldingWeapon` true)
    (else
      (`SceneComponent.SetVisibility` _defaultsceneroot false true)
      (set `self.isHoldingWeapon` true)))
  (`self.ApplyUpgrade`))

(event `self.I_RemoveAndDeleteWeapon`
  (params (`Weapon Class` :type "/Game/Tech/Weapons/WeaponInfo/BP_BaseWeapon Class Reference") (`Inventory Index` :type Integer))
  (bind _output (`|GetArrayItem` (`self.Weapon_Inventory`) `Inventory Index`))
  ;[0 1 1] Get the weapon of selected index and destroy it
  (`KismetSystemLibrary.PrintText` (`|FormatText` "{weapon} removed from slot {x}" (`KismetSystemLibrary.GetClassDisplayName` (`GameplayStatics.GetObjectClass` (`|GetArrayItem` (`self.Weapon_Inventory`) `Inventory Index`))) `Inventory Index`) true true (struct :`R` 0.5 :`B` 0.5 :`A` 1.0) 3.0)
  (bind _returnvalue (`|SpawnActorFromClass` "/Game/Tech/Pickups/BP_WeaponPickupV2.BP_WeaponPickupV2_C" (`KismetMathLibrary.MakeTransform` (+ (`self.K2_GetActorLocation`) (300.0 0.0 0.0))) "AlwaysSpawn" "OverrideRootScale" null null))
  (`/Game/Tech/Pickups/BP_WeaponPickupV2.SpawnInformation` _returnvalue (`.WeaponName_34_C3694ECA427C22994D707E9D808D1F6C` (break `/Game/Tech/Weapons/WeaponInfo/WeaponInformation` (`/Game/Tech/Weapons/WeaponInfo/BP_BaseWeapon.WeaponInformation` _output))))
  (`self.K2_DestroyActor` _output))

(event `ApplyUpgrade`
  (for _array_element (`self.K2_GetComponentsByClass` "/Game/Tech/Upgrades/BPC_BaseUpgrade.BPC_BaseUpgrade_C")
    (if (== (`/Game/Tech/Upgrades/BPC_BaseUpgrade.Slot` _array_element) (`KismetArrayLibrary.Array_Find` (`self.Weapon_Inventory`) (`self.SpawnedWeapon`)))
      (`self.I_InitialiseComponent` (`self.SpawnedWeapon`) (`GameplayStatics.GetObjectClass` _array_element) (`/Game/Tech/Upgrades/BPC_BaseUpgrade.Slot` _array_element)))))

(event `self.I_DestroyComponent`
  (params (Component :type "ActorComponent Object Reference"))
  (`ActorComponent.K2_DestroyComponent` Component))

(event `self.I_InitialiseComponent`
  (params (Component :type "/Game/Tech/Upgrades/BPC_BaseUpgrade Class Reference") (Slot :type Integer))
  (bind _output (`|GetArrayItem` (`self.Weapon_Inventory`) Slot))
  (bind _returnvalue (`|AddComponentByClass` Component Slot))
  (`/Game/Tech/Upgrades/BPC_BaseUpgrade.Upgrade Init` _returnvalue)
  (`/Engine/EditorBlueprintResources/StandardMacros.IsValid` _returnvalue
    (:`Is Valid`
      (`/Game/Tech/Upgrades/BPC_BaseUpgrade.Upgrade_Player` _returnvalue)
      (`/Engine/EditorBlueprintResources/StandardMacros.IsValid` _output
        (:`Is Valid`
          (`self.I_InitialiseComponent` _output Component Slot))))))

(fn `I_ApplyDamage`
  (params (Damage :type "Float (double-precision)") (Instigator :type "Actor Object Reference"))
  (returns (`Target Hit?` :type Boolean) (`Target Dead?` :type Boolean))
  (bind _bpc_healthcomponent (`self.BPC_HealthComponent`))
  ;[0 1 1] Sending damage to health component and updating event dispatcher for UI
  (bind (_target_hit_ _target_dead_) (`/Game/Tech/HealthSystem/BPC_HealthComponent.I_ApplyDamage` _bpc_healthcomponent Damage Instigator))
  (`self.E_HealthUpdated` (`/Game/Tech/HealthSystem/BPC_HealthComponent.S_Health` _bpc_healthcomponent))
  (return _target_hit_ _target_dead_))

(fn `I_ApplyHealing`
  (params (Healing :type "Float (double-precision)") (Instigator :type "Actor Object Reference"))
  (returns (`Target Full?` :type Boolean))
  (bind _bpc_healthcomponent (`self.BPC_HealthComponent`))
  ;[0 1 1] Sending healing to health component and updating event dispatcher for UI
  (bind _target_full_ (`/Game/Tech/HealthSystem/BPC_HealthComponent.I_ApplyHealing` _bpc_healthcomponent Healing Instigator))
  (`self.E_HealthUpdated` (`/Game/Tech/HealthSystem/BPC_HealthComponent.S_Health` _bpc_healthcomponent))
  (return _target_full_))

(fn `I_ChangeMaxHealth`
  (params (`Max Health` :type "Float (double-precision)") (Instigator :type "Actor Object Reference"))
  (returns (`Return Value` :type Boolean))
  (bind _bpc_healthcomponent (`self.BPC_HealthComponent`))
  (bind _return_value (`self.I_ChangeMaxHealth` _bpc_healthcomponent `Max Health` Instigator))
  (`self.E_HealthUpdated` (`/Game/Tech/HealthSystem/BPC_HealthComponent.S_Health` _bpc_healthcomponent))
  (return _return_value))

(fn `I_CheckDuplicateWeapon`
  (params (`Weapon Class` :type "/Game/Tech/Weapons/WeaponInfo/BP_BaseWeapon Class Reference"))
  (returns (`Duplicate?` :type Boolean))
  (locals (`Duplicate Weapon` :type Boolean))
  ;[0 1 1] Check for duplicate weapon - Get weapon class for all weapons and compare with Weapon class input
  (for _array_element (`self.Weapon_Inventory`)
    (bind _output_get (set `local.Duplicate Weapon` (== (`GameplayStatics.GetObjectClass` _array_element) (`local.Weapon Class`))))
    (if _output_get
      (break)))
  (`KismetSystemLibrary.PrintText` (`|FormatText` "Duplicate of {weapon}: {bool}" (`KismetSystemLibrary.GetClassDisplayName` (`local.Weapon Class`)) (`local.Duplicate Weapon`)) true true (struct :`R` 0.5 :`B` 0.5 :`A` 1.0) 3.0)
  (return (`local.Duplicate Weapon`)))

(fn `I_CheckFullInventory`
  (returns (`Full?` :type Boolean))
  (bind _inventorymaxsize (`self.InventoryMaxSize`))
  (bind _returnvalue (`KismetArrayLibrary.Array_Length` (`self.Weapon_Inventory`)))
  ;[0 1 1] Check if inventory is full
  (`KismetSystemLibrary.PrintText` (`|FormatText` "Inventory Full: {bool} \n{current} / {max} slots filled previously" (>= _returnvalue _inventorymaxsize) _returnvalue _inventorymaxsize) true true (struct :`R` 0.5 :`B` 0.5 :`A` 1.0) 3.0)
  (return (>= (`KismetArrayLibrary.Array_Length` (`self.Weapon_Inventory`)) (`self.InventoryMaxSize`))))

(fn `I_GetHealthStruct`
  (returns (`Health Struct` :type "/Game/Tech/HealthSystem/S_Health Structure"))
  (bind _health_struct (`self.I_GetHealthStruct` (`self.BPC_HealthComponent`)))
  (return _health_struct))

(fn `I_PickUpWeapon`
  (params (`Weapon Class` :type "/Game/Tech/Weapons/WeaponInfo/BP_BaseWeapon Class Reference") (Itemslot :type Integer))
  (returns (`Picked Up?` :type Boolean))
  (bind _weapon_class (`local.Weapon Class`))
  ;[0 1 1] When the player picks up a weapon
  ;[0 1 1] Check if the weapon is a duplicate, if the weapon is a dupe, ignore it
  (bind _duplicate_ (`self.I_CheckDuplicateWeapon` `Weapon Class`))
  (if _duplicate_
    (return false)
    (else
      ;[0 1 1] If the weapon isn't a dupe, check if the inventory is full
      (bind _full_ (`self.I_CheckFullInventory`))
      (if _full_
        ;[0 1 1] If the playerss inv is full, drop the current weapon and add the new one
        (`self.I_RemoveAndDeleteWeapon` _weapon_class Itemslot)
        (`self.I_AddAndAttachWeapon` _weapon_class Itemslot)
        (return true)
        (else
          ;[0 1 1] If inv is not full, add the weapon to the players inventory
          (`self.I_AddAndAttachWeapon` (`local.Weapon Class`) (`KismetArrayLibrary.Array_Length` (`self.Weapon_Inventory`)))
          (return true))))))

(fn `Look At Cursor`
  (bind (_worldlocation _worlddirection) (`PlayerController.DeprojectMousePositionToWorld` (`GameplayStatics.GetPlayerController` 0)))
  ;[1 1 1] Drawing a Line Trace from the camera to the Ground
  (if (not (`self.InHubWorld?`))
    (bind (_outhit _returnvalue) (`KismetSystemLibrary.LineTraceSingle` _worldlocation (+ _worldlocation (* _worlddirection (+ (`SpringArmComponent.TargetArmLength` (`self.SpringArm`)) 2000.0))) "TraceTypeQuery1"))
    (if _returnvalue
      ;[1 1 1] Getting The Direction To Look At
      (bind _output_get (set `self.Direction` (`.Location` (`GameplayStatics.BreakHitResult` _outhit))))
      (`self.K2_SetActorRotation` (`KismetMathLibrary.MakeRotator` 0.0 0.0 (.yaw (`KismetMathLibrary.FindLookAtRotation` (`self.K2_GetActorLocation`) _output_get)))))))

(fn `UserConstructionScript`)