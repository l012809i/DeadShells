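; Shell Axe melee weapon, a child weapon Blueprint that passes activation, deactivation and construction to its parent.
; Its attack checks AttackIndex: at the third step or beyond it resets the index and only prints a lunge debug message.
; Otherwise it calls UpgradeMeleeWeapon on every BPC_BaseUpgrade component, passing spawn type, damage and its chain lightning components.
; The index is not incremented here, and the damage and healing message nodes are unconnected.
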(event `self.ActivateWeapon`
  ;[0 1 1] Add custom firing mechanics here
  (`parent.ActivateWeapon`))

(event `self.WeaponFunctionality`
  ;[0 1 1] Add Weapon Functionality Here!
  (if (>= (`self.AttackIndex`) 3)
    (set `self.AttackIndex` 1)
    (`KismetSystemLibrary.PrintString` "lunge")
    (else
      (if (== (`self.AttackIndex`) 1)
        _
        (else
          _))
      (for _array_element (`self.K2_GetComponentsByClass` "/Game/Tech/Upgrades/BPC_BaseUpgrade.BPC_BaseUpgrade_C")
        (`/Game/Tech/Upgrades/BPC_BaseUpgrade.Upgrade_MeleeWeapon` _array_element (`self.Melee Spawn Type`) (`self.F_GetDamage`) (`self.K2_GetComponentsByClass` "/Game/Tech/Upgrades/BPC_ChainLightning.BPC_ChainLightning_C"))
        (`KismetSystemLibrary.PrintString` "attac")))))

(event `self.DeactivateWeapon`
  (params (`Weapon Switch?` :type Boolean))
  ;[0 1 1] Add custom firing mechanics here
  (`parent.DeactivateWeapon` `Weapon Switch?`))

(fn `UserConstructionScript`
  (`parent.UserConstructionScript`))