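; BP_BubbleBomber is a weapon Blueprint that fires a growing burst of bubble projectiles.
; Each WeaponFunctionality call raises BubbleCount, capped at ten, and spawns that many BP_BubbleProjectile actors at the owning player's Projectilespawn.
; Each bubble gets a small random yaw offset, so the burst fans out.
; DeactivateWeapon calls the parent logic and resets the count, restarting the ramp.
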(event `self.WeaponFunctionality`
  (bind _returnvalue (`self.GetOwner`))
  ;[0 1 1] Add Weapon Functionality Here!
  (bind _result (`/Engine/EditorBlueprintResources/StandardMacros.IncrementInt` (`self.Bubble Count`))
    (:`  `
      (bind _output_get (set `self.Bubble Count` (`KismetMathLibrary.Clamp` _result 1 10)))
      (for _ (range 1 (+ _output_get 1))
        (`|SpawnActorFromClass` "/Game/Tech/Projectiles/BP_BubbleProjectile.BP_BubbleProjectile_C" (`KismetMathLibrary.MakeTransform` (.location (`SceneComponent.K2_GetComponentToWorld` (`/Game/Tech/Character/BP_Player.Projectilespawn` (cast `/Game/Tech/Character/BP_Player` _returnvalue :!pure true)))) (`KismetMathLibrary.ComposeRotators` (.rotation (`SceneComponent.K2_GetComponentToWorld` (`/Game/Tech/Character/BP_Player.Projectilespawn` (cast `/Game/Tech/Character/BP_Player` _returnvalue :!pure true)))) (`KismetMathLibrary.MakeRotator` 0.0 0.0 (`KismetMathLibrary.RandomFloatInRange` -10.0 10.0)))) "AlwaysSpawn" "OverrideRootScale" _returnvalue null)))))

(event `self.DeactivateWeapon`
  (params (`Weapon Switch?` :type Boolean))
  (`parent.DeactivateWeapon` false)
  (set `self.Bubble Count` 0))

(fn `UserConstructionScript`
  (`parent.UserConstructionScript`))