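; BP_FishSwordSweep is a short-lived melee attack actor that sweeps a fish sword hit arc along a spline placed ahead of it.
; On BeginPlay a rate-scaled timeline plays forward or in reverse, moving the end of a debug-drawn pawn multi-line trace along the spline.
; Each hit actor receives damage through an interface and is then ignored.
; Registered hits notify BPC_BaseUpgrade components, while unregistered ones destroy the sweep.
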(event `self.ReceiveBeginPlay`
  (bind _spline (`self.Spline`))
  (`parent.ReceiveBeginPlay`)
  (`TimelineComponent.SetPlayRate` (`self.AttackTimeline`) (/ 1.0 0.3))
  (if (`self.Backwards?`)
    (bind (_direction _alpha) (`Timeline|AttackTimeline` :!via `ReverseFromEnd` :!label _label)
      (:`Update`
        (bind _outhits (`KismetSystemLibrary.LineTraceMultiForObjects` (`self.K2_GetActorLocation`) (`SplineComponent.GetLocationAtDistanceAlongSpline` _spline (`KismetMathLibrary.Lerp` 0.0 (`SplineComponent.GetSplineLength` _spline) _alpha) "World") (`|MakeArray` "ObjectTypeQuery3" :!type "EObjectTypeQuery Enum") false (`self.Actors to Ignore`) "ForDuration"))
        (for _array_element _outhits
          (bind (_bblockinghit _binitialoverlap _time _distance _location _impactpoint _normal _impactnormal _physmat _hitactor) (`GameplayStatics.BreakHitResult` _array_element))
          (bind _target_hit_ (message `/Game/Tech/HealthSystem/BPI_DamageHandling.I_ApplyDamage` _hitactor (`self.Damage`) (`self.GetOwner`)))
          (`KismetArrayLibrary.Array_AddUnique` (`self.Actors to Ignore`) _hitactor)
          (if _target_hit_
            (for _array_element_2 (`self.K2_GetComponentsByClass` "/Game/Tech/Upgrades/BPC_BaseUpgrade.BPC_BaseUpgrade_C")
              (`/Game/Tech/Upgrades/BPC_BaseUpgrade.Upgrade_Hit` _array_element_2 (`self.Damage`)))
            (else
              (`self.K2_DestroyActor`))))))
    (else
      (goto _label :!via `PlayFromStart`))))

(fn `UserConstructionScript`
  (`SceneComponent.K2_SetWorldLocation` (`self.Spline`) (+ (`self.K2_GetActorLocation`) (* (`SceneComponent.GetForwardVector` (`self.DefaultSceneRoot`)) (`self.DistanceFromPlayer`))) false true))